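; AI vehicle controller that drives its pawn along one side of a BP_AIPath and handles overtaking.
; Each Tick, it aims at a speed-scaled look-ahead point for steering, while a farther point's angle sets top speed for throttle, braking and brake lights.
; A looping timer checks collision boxes to switch road side around a vehicle in front, or override top speed with that vehicle's when the other side is blocked.
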(event `self.ReceiveBeginPlay`
  (set `self.ControlledVehicle` (`self.K2_GetPawn`))
  (bind _returnvalue (`GameplayStatics.GetActorOfClass` "/Game/AI/BP_AIPath.BP_AIPath_C"))
  (set `self.AIPath` _returnvalue)
  (bind _side_of_road (`self.Calculate Starting Side Of Road`))
  (set `self.Side Of Road` _side_of_road)
  (`KismetSystemLibrary.K2_SetTimer` null "Check For Overtakes" 0.1 true))

(event `self.ReceiveTick`
  (params (DeltaSeconds :type "Float (single-precision)"))
  (bind _steering_input (`self.Calculate Steering`))
  (message `/Game/AI/BPI_IsVehicle.SetSteering` (`self.ControlledVehicle`) _steering_input)
  (bind _top_speed (`self.Calculate Top Speed`))
  (bind (_throttle _brake) (`self.Calculate Throttle/brake` _top_speed))
  (message `/Game/AI/BPI_IsVehicle.SetThrottle` (`self.ControlledVehicle`) _throttle)
  (message `/Game/AI/BPI_IsVehicle.SetBrake` (`self.ControlledVehicle`) _brake)
  (if (>= _brake 0.1)
    (message `/Game/AI/BPI_IsVehicle.SetBrakeLights` (`self.ControlledVehicle`) true)
    (`KismetSystemLibrary.RetriggerableDelay` 0.3)
    (message `/Game/AI/BPI_IsVehicle.SetBrakeLights` (`self.ControlledVehicle`) false)))

(fn `Calculate Starting Side Of Road`
  (returns (`Side Of Road` :type Integer))
  (locals (LeftSideDistance :type "Float (double-precision)" :default 0.0) (RightSideDistance :type "Float (double-precision)" :default 0.0))
  (bind _returnvalue (`self.K2_GetActorLocation` (`self.ControlledVehicle`)))
  (bind _returnvalue_2 (`self.K2_GetActorLocation` (`self.ControlledVehicle`)))
  ;[1 1 1] Get The side of roade based on each side
  (bind _location_to_steer_to (`/Game/AI/BPI_IsAIPath.Get Closest Location to AI Path` (`self.AIPath`) _returnvalue_2 0.0 0))
  (set `local.LeftSideDistance` (`KismetMathLibrary.Vector_Distance` _location_to_steer_to _returnvalue_2))
  (bind _location_to_steer_to_2 (`/Game/AI/BPI_IsAIPath.Get Closest Location to AI Path` (`self.AIPath`) _returnvalue 0.0 1))
  (set `local.RightSideDistance` (`KismetMathLibrary.Vector_Distance` _location_to_steer_to_2 _returnvalue))
  (return (`KismetMathLibrary.Conv_BoolToInt` (> (`local.LeftSideDistance`) (`local.RightSideDistance`)))))

(fn `Calculate Steering`
  (returns (`Steering Input` :type "Float (double-precision)"))
  ;[1 1 1] Get the closest poin to the spline
  (bind _currentspeed (message `/Game/AI/BPI_IsVehicle.GetCurrentSpeed` (`self.ControlledVehicle`)))
  (bind _front_location (message `/Game/AI/BPI_IsVehicle.GetFrontOfCar` (`self.ControlledVehicle`)))
  (bind _location_to_steer_to (message `/Game/AI/BPI_IsAIPath.Get Closest Location to AI Path` (`self.AIPath`) _front_location (`KismetMathLibrary.MapRangeClamped` _currentspeed 50.0 150.0 1000.0 3000.0) (`self.Side Of Road`)))
  (bind (_returnvalue_roll _returnvalue_pitch _returnvalue_yaw) (`KismetMathLibrary.BreakRotator` (`KismetMathLibrary.NormalizedDeltaRotator` (`KismetMathLibrary.FindLookAtRotation` _front_location _location_to_steer_to) (`self.K2_GetActorRotation` (`self.ControlledVehicle`)))))
  (return (`KismetMathLibrary.MapRangeClamped` _returnvalue_yaw -10.0 10.0 -1.0 1.0)))

(fn `Calculate Throttle/brake`
  (params (`Top Speed` :type "Float (double-precision)"))
  (returns (Throttle :type "Float (double-precision)") (Brake :type "Float (double-precision)"))
  (locals (CurrentSpeed :type "Float (double-precision)" :default 0.0))
  (bind _top_speed (`local.Top Speed`))
  (bind _currentspeed (message `/Game/AI/BPI_IsVehicle.GetCurrentSpeed` (`self.ControlledVehicle`)))
  (bind _output_get (set `local.CurrentSpeed` _currentspeed))
  (if (>= _output_get (`local.Top Speed`))
    (return 0.0 (`KismetMathLibrary.MapRangeClamped` (`local.CurrentSpeed`) (+ _top_speed 1.0) (+ _top_speed 5.0) 0.0 1.0))
    (else
      (return 1.0 0.0))))

(fn `Calculate Top Speed`
  (returns (`Top Speed` :type "Float (double-precision)"))
  (if (`self.Override Top Speed?`)
    (return (`self.Override Top Speed`))
    (else
      ;[1 1 1] Get the closest poin to the spline
      (bind _currentspeed (message `/Game/AI/BPI_IsVehicle.GetCurrentSpeed` (`self.ControlledVehicle`)))
      (bind _front_location (message `/Game/AI/BPI_IsVehicle.GetFrontOfCar` (`self.ControlledVehicle`)))
      (bind _location_to_steer_to (message `/Game/AI/BPI_IsAIPath.Get Closest Location to AI Path` (`self.AIPath`) _front_location (`KismetMathLibrary.MapRangeClamped` _currentspeed 50.0 150.0 3000.0 9000.0) (`self.Side Of Road`)))
      (bind (_returnvalue_roll _returnvalue_pitch _returnvalue_yaw) (`KismetMathLibrary.BreakRotator` (`KismetMathLibrary.NormalizedDeltaRotator` (`KismetMathLibrary.FindLookAtRotation` _front_location _location_to_steer_to) (`self.K2_GetActorRotation` (`self.ControlledVehicle`)))))
      (return (`KismetMathLibrary.MapRangeClamped` (`KismetMathLibrary.Abs` _returnvalue_yaw) 0.0 40.0 150.0 50.0)))))

(fn `Check For Overtakes`
  (locals (`Vehicle In Front?` :type Boolean) (VehicleInFront :type "Actor Object Reference") (`Vehicle In Right Side?` :type Boolean) (`Vehicle In Left Side?` :type Boolean))
  (`|ExecutionSequence`
    (:`then_0`
      (bind _front_box (message `/Game/AI/BPI_IsVehicle.Get Collision Boxes` (`self.ControlledVehicle`)))
      (bind _overlappingactors (`PrimitiveComponent.GetOverlappingActors` _front_box null))
      (bind _returnvalue (> (`KismetArrayLibrary.Array_Length` _overlappingactors) 0))
      (if _returnvalue
        (set `local.Vehicle In Front?` _returnvalue)
        (set `local.VehicleInFront` (`|GetArrayItem` _overlappingactors))
        (else
          (set `self.Override Top Speed?` false))))
    (:`then_1`
      (if (`local.Vehicle In Front?`)
        (if (`KismetMathLibrary.Conv_IntToBool` (`self.Side Of Road`))
          (bind (_front_box_2 _left_side_box) (message `/Game/AI/BPI_IsVehicle.Get Collision Boxes` (`self.ControlledVehicle`)))
          (bind _returnvalue_2 (> (`KismetArrayLibrary.Array_Length` (`PrimitiveComponent.GetOverlappingActors` _left_side_box null)) 0))
          (if _returnvalue_2
            (set `local.Vehicle In Left Side?` _returnvalue_2)
            (else
              (set `self.Override Top Speed?` false)))
          (else
            (bind (_front_box_3 _left_side_box_2 _right_side_box) (message `/Game/AI/BPI_IsVehicle.Get Collision Boxes` (`self.ControlledVehicle`)))
            (bind _returnvalue_3 (> (`KismetArrayLibrary.Array_Length` (`PrimitiveComponent.GetOverlappingActors` _right_side_box null)) 0))
            (if _returnvalue_3
              (set `local.Vehicle In Right Side?` _returnvalue_3)
              (else
                (set `self.Override Top Speed?` false)))))
        (else
          (set `self.Override Top Speed?` false))))
    (:`then_2`
      (if (and (`local.Vehicle In Front?`) (or (`local.Vehicle In Right Side?`) (`local.Vehicle In Left Side?`)))
        (set `self.Override Top Speed?` (< (`KismetMathLibrary.Vector_Distance` (`self.K2_GetActorLocation` (`self.ControlledVehicle`)) (`self.K2_GetActorLocation` (`local.VehicleInFront`))) 750.0))
        (bind _currentspeed (message `/Game/AI/BPI_IsVehicle.GetCurrentSpeed` (`local.VehicleInFront`)))
        (set `self.Override Top Speed` _currentspeed)
        (elif (`local.Vehicle In Front?`)
          (set `self.Override Top Speed?` false)
          (set `self.Side Of Road` (`KismetMathLibrary.SelectInt` 0 1 (`KismetMathLibrary.Conv_IntToBool` (`self.Side Of Road`))))
          (else
            (set `self.Override Top Speed?` false)))))))

(fn `UserConstructionScript`)